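; Air hockey table actor that acts as the player's view and lets the mouse control a mallet.
; On BeginPlay it becomes the view target of the first player controller.
; Each tick it deprojects the mouse position and runs a short visibility line trace into the world.
; On a hit, the Mallet component jumps to the hit location without sweeping for collision.
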(event EventBeginPlay
  (Game|Player|SetViewTargetwithBlend (Game|GetPlayerController 0) self 0.0 "VTBlend_Linear" 0.0 false))

(event EventTick
  (params (DeltaSeconds :type Float%20%28single-precision%29))
  (bind _returnvalue (Game|GetPlayerController 0))
  (bind (_worldlocation _worlddirection) (Game|Player|ConvertMouseLocationToWorldSpace _returnvalue))
  (bind (_outhit _returnvalue_2) (Collision|LineTraceByChannel _worldlocation (+ _worldlocation (* _worlddirection 8e+02)) "TraceTypeQuery1" false 0 "None"))
  (if _returnvalue_2
    (Transformation|SetWorldLocation (Variables|Default|GetMallet) (.Location (Collision|BreakHitResult _outhit)) false)))

(fn ConstructionScript)